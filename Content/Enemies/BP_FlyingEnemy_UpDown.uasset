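; Flying enemy that patrols vertically and makes ranged attacks on the player cat.
; HandleFlying moves it up or down, using line traces for ceiling and floor to pause and reverse direction, and skips movement while damaged or attacking.
; AttackingCat flips it to face the player along X, waits out the attack animation, then calls Attack, with a DoOnce cooldown gating repeats.
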(event EventBeginPlay
  (|CallParentFunction) ; This node is disabled and will not be called.\nDrag off pins to build functionality.
)

(event Collision|EventActorBeginOverlap
  (params (OtherActor :type Actor%20Object%20Reference)))

(event EventTick
  (params (DeltaSeconds :type Float%20%28single-precision%29))
  (|CallParentFunction DeltaSeconds) ; This node is disabled and will not be called.\nDrag off pins to build functionality.
)

(event EventHandleFlying
  (bind _returnvalue (Transformation|GetActorLocation))
  (bind _returnvalue_2 (Transformation|GetActorLocation))
  (if (not (Variables|Default|GetEnemyDead?))
    (Utilities|FlowControl|Sequence
      (:then_1
        (if (not (or (Variables|Default|GetEnemyDamaged?) (Variables|Default|GetRangedAttacking?)))
          (Pawn|Input|AddMovementInput "0.000000, 0,1.000000" (Variables|Default|GetFlyingDirection) false)
          (if (> (Variables|Default|GetFlyingDirection) 0.0)
            ;[1 1 1] Check for ceiling
            (bind _returnvalue_3 (Collision|LineTraceByChannel _returnvalue_2 (+ _returnvalue_2 (* (Transformation|GetActorUpVector) (Math|Vector|MakeVector 0.0 0.0 2e+02))) "TraceTypeQuery1" false 0 "ForDuration"))
            (if _returnvalue_3
              (Variables|/Script/Engine.CharacterMovementComponent|SetMaxWalkSpeed (Variables|Character|GetCharacterMovement) 0.0)
              (Utilities|FlowControl|Delay (Variables|Default|GetWaitTime))
              (Variables|/Script/Engine.CharacterMovementComponent|SetMaxWalkSpeed (Variables|Character|GetCharacterMovement) (Variables|Default|GetE_Walk%20Speed))
              (Variables|Default|SetFlyingDirection (* (Variables|Default|GetFlyingDirection) -1.0)))
            (else
              ;[1 1 1] Check for floor
              (bind _returnvalue_4 (Collision|LineTraceByChannel _returnvalue (+ (- _returnvalue "0,0,200.000000") (* (Transformation|GetActorUpVector) (Math|Vector|MakeVector 0.0 0.0 -2e+02))) "TraceTypeQuery1" false 0 "ForDuration"))
              (if _returnvalue_4
                (Variables|/Script/Engine.CharacterMovementComponent|SetMaxWalkSpeed (Variables|Character|GetCharacterMovement) 0.0)
                (Utilities|FlowControl|Delay (Variables|Default|GetWaitTime))
                (Variables|/Script/Engine.CharacterMovementComponent|SetMaxWalkSpeed (Variables|Character|GetCharacterMovement) (Variables|Default|GetE_Walk%20Speed))
                (Variables|Default|SetFlyingDirection (* (Variables|Default|GetFlyingDirection) -1.0))))))))))

(event EventAttackingCat
  (if (not (Variables|Default|GetEnemyDead?))
    (CallFunction|RotateTowardsCat)
    (Utilities|FlowControl|DoOnce false :!label _label
      (:Completed
        (Variables|Default|SetRangedAttacking? true)
        (Utilities|FlowControl|Delay (Class|PaperFlipbook|GetTotalDuration (Variables|Default|GetE_Ranged%20Attack)))
        (CallFunction|Attack)
        (Variables|Default|SetRangedAttacking? false)
        (Utilities|FlowControl|Delay (Variables|Default|GetCoolDownDuration))
        (goto _label Reset)))))

(fn ConstructionScript
  (|CallParentFunction))

(fn RotateTowardsCat
  (if (< (.x (Math|Vector|Normalize (Math|Vector|GetUnitDirection(Vector) (Transformation|GetActorLocation (Game|GetPlayerCharacter 0)) (Transformation|GetActorLocation)))) 0.0)
    (Transformation|SetActorRotation "0,180.000000,0.000000")
    (Variables|Default|SetIsTurnedRight? true)
    (else
      (Transformation|SetActorRotation "0, 0, 0")
      (Variables|Default|SetIsTurnedRight? false))))