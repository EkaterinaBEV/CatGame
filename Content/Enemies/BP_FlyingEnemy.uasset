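; Flying 2D enemy that patrols horizontally, reversing after a pause at walls, and fires bomb projectiles at the player cat.
; BeginPlay loads flipbooks and health from Enemy_DT by EnemyType; Tick drives animation, movement and sphere-trace detection.
; Detection triggers a cooldown-gated attack aimed at the player.
; Stomps bounce the cat and other hits launch the enemy; both reduce health, leading to a death animation and destruction.
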(event OnComponentBeginOverlap(JumpOnBox)
  (params (OverlappedComponent :type Primitive%20Component%20Object%20Reference) (OtherActor :type Actor%20Object%20Reference) (OtherComp :type Primitive%20Component%20Object%20Reference) (OtherBodyIndex :type Integer) (bFromSweep :type Boolean) (SweepResult :type Hit%20Result%20Structure%20%28by%20ref%29))
  ;[1 1 1] JumpedOn
  (bind _asbp_cat (Utilities|Casting|CastToBP_Cat OtherActor))
  (if (AI|Components|NavMovement|IsFalling (Variables|/Script/Engine.Character|GetCharacterMovement _asbp_cat))
    (Variables|Checks|SetEnemyDamaged? true)
    (CallFunction|ChangeHealth _asbp_cat)
    (CallFunction|JumpDamage)
    (Character|LaunchCharacter _asbp_cat "0, 0,500.000000" true true)))

(event Custom|HandleAnimation
  (bind _e_dying (Variables|Animation|GetE_Dying))
  ;[1 1 1] Animation
  (if (Variables|Checks|GetEnemyDead?)
    (Sprite|SetFlipbook (Variables|Default|GetSprite) _e_dying)
    (Utilities|FlowControl|Delay (Class|PaperFlipbook|GetTotalDuration _e_dying))
    (Actor|DestroyActor self)
    (elif (Variables|Checks|GetEnemyDamaged?)
      (Sprite|SetFlipbook (Variables|Default|GetSprite) (Variables|Animation|GetE_Damaged))
      (elif (Variables|Checks|GetRangedAttacking?)
        (Sprite|SetFlipbook (Variables|Default|GetSprite) (Variables|Animation|GetE_Ranged%20Attack))
        (else
          (Sprite|SetFlipbook (Variables|Default|GetSprite) (select (> (Math|Vector|VectorLength (Variables|/Script/Engine.MovementComponent|GetVelocity (Variables|Character|GetCharacterMovement))) 0.0) (Variables|Animation|GetE_Moving) (Variables|Animation|GetE_Idle))))))))

(event Custom|AttackingCat
  ;[1 1 1] Enemy Attack
  (if (not (Variables|Checks|GetEnemyDead?))
    (Utilities|FlowControl|DoOnce false :!label _label
      (:Completed
        (Variables|Checks|SetRangedAttacking? true)
        (Utilities|FlowControl|Delay (Class|PaperFlipbook|GetTotalDuration (Variables|Animation|GetE_Ranged%20Attack)))
        (CallFunction|Attack)
        (Variables|Checks|SetRangedAttacking? false)
        (Utilities|FlowControl|Delay (Variables|Default|GetCoolDownDuration))
        (goto _label Reset)))))

(event Custom|JumpDamage
  ;[1 1 1] OnDamaged
  (Utilities|FlowControl|RetriggerableDelay (Class|PaperFlipbook|GetTotalDuration (Variables|Animation|GetE_Damaged)))
  (Variables|Checks|SetEnemyDamaged? false))

(event Custom|HandleFlying
  (bind _returnvalue (Transformation|GetActorLocation))
  (if (not (Variables|Checks|GetEnemyDead?))
    (Utilities|FlowControl|Sequence
      (:then_0
        (if (> (Variables|Default|GetMovementDirection) 0.0)
          (Transformation|SetActorRotation "0,180.000000, 0")
          (else
            (Transformation|SetActorRotation "0, 0, 0"))))
      (:then_1
        (if (not (or (Variables|Checks|GetEnemyDamaged?) (Variables|Checks|GetRangedAttacking?)))
          (Pawn|Input|AddMovementInput "1.000000, 0, 0" (Variables|Default|GetMovementDirection) false)
          ;[1 1 1] Check for wall
          (bind _returnvalue_2 (Collision|LineTraceByChannel _returnvalue (+ _returnvalue (* (Transformation|GetActorForwardVector) (Math|Vector|MakeVector -1.5e+02 0.0 0.0))) "TraceTypeQuery1" false 0 "None"))
          (if _returnvalue_2
            (Utilities|FlowControl|DoOnce false :!label _label
              (:Completed
                (Variables|/Script/Engine.CharacterMovementComponent|SetMaxWalkSpeed (Variables|Character|GetCharacterMovement) 0.0)
                (Utilities|FlowControl|Delay (Variables|Default|GetWaitTime))
                (Variables|/Script/Engine.CharacterMovementComponent|SetMaxWalkSpeed (Variables|Character|GetCharacterMovement) (Variables|Default|GetE_Walk%20Speed))
                (Variables|Default|SetMovementDirection (* (Variables|Default|GetMovementDirection) -1.0))
                (goto _label Reset)))))))))

(event EventBeginPlay
  (Variables|/Script/Engine.CharacterMovementComponent|SetMaxWalkSpeed (Variables|Character|GetCharacterMovement) (Variables|Default|GetE_Walk%20Speed))
  (CallFunction|SetEnemyData))

(event Game|Damage|EventAnyDamage
  (params (Damage :type Float%20%28single-precision%29) (DamageType :type Damage%20Type%20Object%20Reference) (InstigatedBy :type Controller%20Object%20Reference) (DamageCauser :type Actor%20Object%20Reference))
  ;[1 1 1] OnDamaged
  (Variables|Checks|SetEnemyDamaged? true)
  (CallFunction|ChangeHealth (.AsBP%20Cat (Utilities|Casting|CastToBP_Cat DamageCauser)))
  ;;[1 1 1] Enemy Thrown Away From Character
  (Character|LaunchCharacter (Math|Vector|MakeVector (* (select (< (.x (Math|Vector|Normalize (Math|Vector|GetUnitDirection(Vector) (Transformation|GetActorLocation DamageCauser) (Transformation|GetActorLocation)))) 0.0) 1.0 -1.0) -5e+02) 0.0 0.0) true true)
  (Utilities|FlowControl|RetriggerableDelay (Class|PaperFlipbook|GetTotalDuration (Variables|Animation|GetE_Damaged)))
  (Variables|Checks|SetEnemyDamaged? false))

(event EventTick
  (params (DeltaSeconds :type Float%20%28single-precision%29))
  (CallFunction|HandleAnimation)
  (CallFunction|HandleFlying)
  (CallFunction|DetectCat))

(fn ConstructionScript)

(fn SetEnemyData
  (bind _outrownames (DataTable|GetDataTableRowNames "/Game/Enemies/Enemy_DT.Enemy_DT"))
  (for _array_element _outrownames
    (bind _returnvalue (Utilities|GetDataTableRow "/Game/Enemies/Enemy_DT.Enemy_DT" _array_element)
      (:then
        (if (Utilities|Enum|Equal(Enum) (Variables|Default|GetEnemyType) (.enemytype _returnvalue))
          (Variables|Animation|SetE_Idle (.idle _returnvalue))
          (Variables|Animation|SetE_Moving (.moving _returnvalue))
          (Variables|Animation|SetE_Attack (.attack _returnvalue))
          (Variables|Animation|SetE_Ranged%20Attack (.rangedattack _returnvalue))
          (Variables|Animation|SetE_Damaged (.damaged _returnvalue))
          (Variables|Animation|SetE_Dying (.dying _returnvalue))
          (Variables|Animation|SetE_Dead (.dead _returnvalue))
          (Variables|Default|SetEnemy%20Health (.enemyhealth _returnvalue)))))))

(fn ChangeHealth
  (params (Cat :type BP%20Cat%20Object%20Reference))
  (if (AI|Components|NavMovement|IsFalling (Variables|/Script/Engine.Character|GetCharacterMovement Cat))
    (bind _output_get (Variables|Default|SetEnemy%20Health (- (Variables|Default|GetEnemy%20Health) (Variables|/Game/Cat/BP_Cat.BP_Cat_C|GetJumpDamage Cat))))
    (Development|PrintString (Utilities|String|ToString(Float) _output_get))
    (else
      (bind _output_get_2 (Variables|Default|SetEnemy%20Health (- (Variables|Default|GetEnemy%20Health) (Variables|/Game/Cat/BP_Cat.BP_Cat_C|GetMeleeDamage Cat))))
      (Development|PrintString (Utilities|String|ToString(Float) _output_get_2))))
  (CallFunction|Dead?))

(fn Dead?
  (if (<= (Variables|Default|GetEnemy%20Health) 0.0)
    (Variables|Checks|SetEnemyDead? true))
  (return))

(fn DetectCat
  (bind _returnvalue (Transformation|GetActorLocation))
  (bind _outhit (Collision|SphereTraceForObjects _returnvalue (+ _returnvalue (+ (Transformation|GetActorForwardVector) (Math|Vector|MakeVector -5e+02 0.0 0.0))) 5e+02 (Utilities|Array|MakeArray "ObjectTypeQuery3") false (Utilities|Array|MakeArray self) "None"))
  (bind _asbp_cat (Utilities|Casting|CastToBP_Cat (.HitActor (Collision|BreakHitResult _outhit))))
  (if (== _asbp_cat (.HitActor (Collision|BreakHitResult _outhit)))
    (Variables|Checks|SetCatDetected? true)
    (CallFunction|AttackingCat)
    (else
      (Variables|Checks|SetCatDetected? false))))

(fn Attack
  (Game|SpawnActorfromClass "/Game/Enemies/Pigeon/Projectile/Bomb_Projectile.Bomb_Projectile_C" (Math|Transform|MakeTransform (Transformation|GetWorldLocation (Variables|Default|GetPojectSpawnLoc)) (Math|Rotator|FindLookatRotation (Transformation|GetActorLocation) (Transformation|GetActorLocation (Game|Player|GetPlayerPawn 0)))) "Undefined" 0 0))