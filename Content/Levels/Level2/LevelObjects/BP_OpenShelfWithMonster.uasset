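; BP_OpenShelfWithMonster is a Level 2 shelf object that spawns a monster and reacts to the cat's presence.
; On BeginPlay it spawns a BP_Enemy at the location of its Scene component.
; When BP_Cat enters the Box trigger, Plane collision turns off after a short random delay.
; When the cat leaves, collision returns to query and physics after a fixed delay.
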(event OnComponentBeginOverlap(Box)
  (params (OverlappedComponent :type Primitive%20Component%20Object%20Reference) (OtherActor :type Actor%20Object%20Reference) (OtherComp :type Primitive%20Component%20Object%20Reference) (OtherBodyIndex :type Integer) (bFromSweep :type Boolean) (SweepResult :type Hit%20Result%20Structure%20%28by%20ref%29))
  (Utilities|Casting|CastToBP_Cat OtherActor)
  (Utilities|FlowControl|Delay (Math|Random|RandomFloatinRange 0.5 1.0))
  (Collision|SetCollisionEnabled (Variables|Default|GetPlane) "NoCollision"))

(event OnComponentEndOverlap(Box)
  (params (OverlappedComponent :type Primitive%20Component%20Object%20Reference) (OtherActor :type Actor%20Object%20Reference) (OtherComp :type Primitive%20Component%20Object%20Reference) (OtherBodyIndex :type Integer))
  (Utilities|Casting|CastToBP_Cat OtherActor)
  (Utilities|FlowControl|Delay 0.5)
  (Collision|SetCollisionEnabled (Variables|Default|GetPlane) "QueryAndPhysics"))

(event EventBeginPlay
  (Game|SpawnActorfromClass "/Game/Enemies/BP_Enemy.BP_Enemy_C" (Math|Transform|MakeTransform (.location (Transformation|GetWorldTransform (Variables|Default|GetScene))) "0, 0, 0" "1.000000,1.000000,1.000000") "Undefined" 0 -1.0 -1.0 false 0))

(fn ConstructionScript)