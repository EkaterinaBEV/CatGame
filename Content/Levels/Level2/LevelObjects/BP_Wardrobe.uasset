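; BP_Wardrobe is a Level 2 object that chains copies of itself as the player's cat reaches it.
; It caches the BP_Cat player on BeginPlay and checks overlaps on the SpawnNewBox trigger against it.
; After a short delay, it spawns another wardrobe at the Arrow's location and scale, plus a GreySquareSpawn at SpawnGreyPlank0.
; It then destroys the trigger component, leaving the wardrobe in place.
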(event OnComponentBeginOverlap(SpawnNewBox)
  (params (OverlappedComponent :type Primitive%20Component%20Object%20Reference) (OtherActor :type Actor%20Object%20Reference) (OtherComp :type Primitive%20Component%20Object%20Reference) (OtherBodyIndex :type Integer) (bFromSweep :type Boolean) (SweepResult :type Hit%20Result%20Structure%20%28by%20ref%29))
  (bind _arrow (Variables|Default|GetArrow))
  (bind _returnvalue (Transformation|GetWorldTransform _arrow))
  (if (== OtherActor (Variables|Default|GetAs%20BP%20Cat))
    (Utilities|FlowControl|Delay 0.2)
    (Game|SpawnActorfromClass "BP_Wardrobe_C" (Math|Transform|MakeTransform (.location _returnvalue) "0, 0, 0" (.scale _returnvalue)) "Undefined" 0 0)
    (Game|SpawnActorfromClass "/Game/GreySquareSpawn.GreySquareSpawn_C" (Math|Transform|MakeTransform (.location (Transformation|GetWorldTransform (Variables|Default|GetSpawnGreyPlank_0))) "0, 0, 0" "1.000000,1.000000,1.000000") "Undefined" 0 0)
    (Components|DestroyComponent (Variables|Default|GetSpawnNewBox))))

(event EventBeginPlay
  (bind _asbp_cat (Utilities|Casting|CastToBP_Cat (Game|GetPlayerCharacter 0)))
  (Variables|Default|SetAs%20BP%20Cat _asbp_cat))

(event Collision|EventActorBeginOverlap
  (params (OtherActor :type Actor%20Object%20Reference)))

(event EventTick
  (params (DeltaSeconds :type Float%20%28single-precision%29)))

(fn ConstructionScript)