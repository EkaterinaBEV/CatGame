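; Level 2 flipbook enemy that walks constantly along -X and fights the player's BP_Cat.
; BeginPlay loads animations and health from Enemy_DT by EnemyType; Tick picks flipbooks from damaged, attacking and dead flags, destroying it after dying.
; CatDetector overlap runs a looping timer into a DoOnce cooldown-gated attack that line-traces to apply melee damage.
; Falling onto JumpOnBox bounces the cat and deals jump damage; other hits use AnyDamage.
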(event OnComponentBeginOverlap(JumpOnBox)
  (params (OverlappedComponent :type Primitive%20Component%20Object%20Reference) (OtherActor :type Actor%20Object%20Reference) (OtherComp :type Primitive%20Component%20Object%20Reference) (OtherBodyIndex :type Integer) (bFromSweep :type Boolean) (SweepResult :type Hit%20Result%20Structure%20%28by%20ref%29))
  ;[1 1 1] JumpedOn
  (bind _asbp_cat (Utilities|Casting|CastToBP_Cat OtherActor))
  (if (AI|Components|NavMovement|IsFalling (Variables|/Script/Engine.Character|GetCharacterMovement _asbp_cat))
    (Variables|Checks|SetEnemyDamaged? true)
    (CallFunction|ChangeHealth _asbp_cat)
    (CallFunction|JumpDamage)
    (Character|LaunchCharacter _asbp_cat "0, 0,500.000000" true true)))

(event OnComponentBeginOverlap(CatDetector)
  (params (OverlappedComponent :type Primitive%20Component%20Object%20Reference) (OtherActor :type Actor%20Object%20Reference) (OtherComp :type Primitive%20Component%20Object%20Reference) (OtherBodyIndex :type Integer) (bFromSweep :type Boolean) (SweepResult :type Hit%20Result%20Structure%20%28by%20ref%29))
  ;[1 1 1] Enemy Attack
  (bind _asbp_cat (Utilities|Casting|CastToBP_Cat OtherActor))
  (if (not (Variables|/Game/Cat/BP_Cat.BP_Cat_C|GetIsDead? _asbp_cat))
    (bind _returnvalue (Utilities|Time|SetTimerbyEvent (delegate Custom|AttackCat) 0.1 true))
    (Variables|Default|SetAttackEvent _returnvalue)))

(event OnComponentEndOverlap(CatDetector)
  (params (OverlappedComponent :type Primitive%20Component%20Object%20Reference) (OtherActor :type Actor%20Object%20Reference) (OtherComp :type Primitive%20Component%20Object%20Reference) (OtherBodyIndex :type Integer))
  (bind _returnvalue (Transformation|GetActorLocation))
  ;[1 1 1] Enemy Attack
  (Utilities|Casting|CastToBP_Cat OtherActor)
  (Utilities|Time|ClearandInvalidateTimerbyHandle (Variables|Default|GetAttackEvent))
  (Utilities|FlowControl|DoOnce false) ; enters at Reset
)

(event Custom|HandleAnimation
  (bind _e_dying (Variables|Animation|GetE_Dying))
  ;[1 1 1] Animation
  (if (Variables|Checks|GetEnemyDead?)
    (Sprite|SetFlipbook (Variables|Default|GetSprite) _e_dying)
    (Utilities|FlowControl|Delay (Class|PaperFlipbook|GetTotalDuration _e_dying))
    (Actor|DestroyActor self)
    (elif (Variables|Checks|GetEnemyDamaged?)
      (Sprite|SetFlipbook (Variables|Default|GetSprite) (Variables|Animation|GetE_Damaged))
      (elif (Variables|Checks|GetEnemyAttacking?)
        (Sprite|SetFlipbook (Variables|Default|GetSprite) (Variables|Animation|GetE_Attack))
        (else
          (Sprite|SetFlipbook (Variables|Default|GetSprite) (Variables|Animation|GetE_Moving)))))))

(event Custom|HandleMovement
  ;[1 1 1] Movement
  (Pawn|Input|AddMovementInput "1.000000, 0, 0" -1.0 false))

(event Custom|JumpDamage
  ;[1 1 1] OnDamaged
  (Utilities|FlowControl|RetriggerableDelay (Class|PaperFlipbook|GetTotalDuration (Variables|Animation|GetE_Damaged)))
  (Variables|Checks|SetEnemyDamaged? false))

(event Custom|AttackCat
  (bind _returnvalue (Transformation|GetActorLocation))
  ;[1 1 1] Enemy Attack
  (if (not (Variables|Checks|GetEnemyDead?))
    (Utilities|FlowControl|DoOnce false :!label _label
      (:Completed
        (Variables|Checks|SetEnemyAttacking? true)
        (Utilities|FlowControl|Delay (Class|PaperFlipbook|GetTotalDuration (Variables|Animation|GetE_Attack)))
        (Utilities|FlowControl|Sequence
          (:then_0
            (Variables|Checks|SetEnemyAttacking? false))
          (:then_1
            (bind _outhit (Collision|LineTraceForObjects _returnvalue (+ _returnvalue (* (Transformation|GetActorForwardVector) (Math|Vector|MakeVector -3.5e+02 0.0 0.0))) (Utilities|Array|MakeArray "ObjectTypeQuery3") false (Utilities|Array|MakeArray self) "ForDuration"))
            (if (== (Game|GetPlayerCharacter 0) (.HitActor (Collision|BreakHitResult _outhit)))
              (Game|Damage|ApplyDamage (.HitActor (Collision|BreakHitResult _outhit)) (Variables|Default|GetMeleeAttackDamage) 0 0))
            (Utilities|FlowControl|Delay (Variables|Default|GetCoolDownDuration))
            (goto _label Reset)))))))

(event EventBeginPlay
  (CallFunction|SetEnemyData))

(event Game|Damage|EventAnyDamage
  (params (Damage :type Float%20%28single-precision%29) (DamageType :type Damage%20Type%20Object%20Reference) (InstigatedBy :type Controller%20Object%20Reference) (DamageCauser :type Actor%20Object%20Reference))
  ;[1 1 1] OnDamaged
  (Variables|Checks|SetEnemyDamaged? true)
  (CallFunction|ChangeHealth (.AsBP%20Cat (Utilities|Casting|CastToBP_Cat DamageCauser)))
  (Utilities|FlowControl|RetriggerableDelay (Class|PaperFlipbook|GetTotalDuration (Variables|Animation|GetE_Damaged)))
  (Variables|Checks|SetEnemyDamaged? false))

(event EventTick
  (params (DeltaSeconds :type Float%20%28single-precision%29))
  (CallFunction|HandleAnimation)
  (CallFunction|HandleMovement))

(fn ConstructionScript)

(fn SetEnemyData
  (bind _outrownames (DataTable|GetDataTableRowNames "/Game/Enemies/Enemy_DT.Enemy_DT"))
  (for _array_element _outrownames
    (bind _returnvalue (Utilities|GetDataTableRow "/Game/Enemies/Enemy_DT.Enemy_DT" _array_element)
      (:then
        (if (Utilities|Enum|Equal(Enum) (Variables|Default|GetEnemyType) (.enemytype _returnvalue))
          (Variables|Animation|SetE_Idle (.idle _returnvalue))
          (Variables|Animation|SetE_Moving (.moving _returnvalue))
          (Variables|Animation|SetE_Attack (.attack _returnvalue))
          (Variables|Animation|SetE_Ranged%20Attack (.rangedattack _returnvalue))
          (Variables|Animation|SetE_Damaged (.damaged _returnvalue))
          (Variables|Animation|SetE_Dying (.dying _returnvalue))
          (Variables|Animation|SetE_Dead (.dead _returnvalue))
          (Variables|Default|SetEnemy%20Health (.enemyhealth _returnvalue)))))))

(fn ChangeHealth
  (params (Cat :type BP%20Cat%20Object%20Reference))
  (if (AI|Components|NavMovement|IsFalling (Variables|/Script/Engine.Character|GetCharacterMovement Cat))
    (bind _output_get (Variables|Default|SetEnemy%20Health (- (Variables|Default|GetEnemy%20Health) (Variables|/Game/Cat/BP_Cat.BP_Cat_C|GetJumpDamage Cat))))
    (Development|PrintString (Utilities|String|ToString(Float) _output_get))
    (else
      (bind _output_get_2 (Variables|Default|SetEnemy%20Health (- (Variables|Default|GetEnemy%20Health) (Variables|/Game/Cat/BP_Cat.BP_Cat_C|GetMeleeDamage Cat))))
      (Development|PrintString (Utilities|String|ToString(Float) _output_get_2))))
  (CallFunction|Dead?))

(fn Dead?
  (if (<= (Variables|Default|GetEnemy%20Health) 0.0)
    (Variables|Checks|SetEnemyDead? true))
  (return))