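; Interactable cat bowl Blueprint that restores a cat's health when used.
; Its Interract function adds Vitality to the cat's Health only while Health is below a fixed threshold, without clamping the result.
; A successful use sets InterractionCompleted, and the function returns the bowl itself in either case.
; Tick and the construction script only call their parent versions.
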(event EventBeginPlay
  (|CallParentFunction) ; This node is disabled and will not be called.\nDrag off pins to build functionality.
)

(event Collision|EventActorBeginOverlap
  (params (OtherActor :type Actor%20Object%20Reference))
  (|CallParentFunction OtherActor) ; This node is disabled and will not be called.\nDrag off pins to build functionality.
)

(event EventTick
  (params (DeltaSeconds :type Float%20%28single-precision%29))
  (|CallParentFunction DeltaSeconds))

(fn ConstructionScript
  (|CallParentFunction))

(fn Interract
  (params (Cat :type BP%20Cat%20Object%20Reference))
  (if (>= (Variables|/Game/Cat/BP_Cat.BP_Cat_C|GetHealth Cat) 9.0)
    _
    (else
      (Variables|/Game/Cat/BP_Cat.BP_Cat_C|SetHealth Cat (+ (Variables|/Game/Cat/BP_Cat.BP_Cat_C|GetHealth Cat) (Variables|Default|GetVitality)))
      (Variables|Default|SetInterractionCompleted? true)))
  (return self))