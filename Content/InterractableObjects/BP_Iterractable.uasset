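; BP_Iterractable is an interactable sprite object that highlights when the cat is near and can be removed after interaction.
; Sphere overlaps with BP_Cat toggle IsCatNear, and SetHighlight swaps the PaperSprite to an Emission material or clears that override.
; Interract prints the object's name, sets InterractionCompleted and returns itself.
; DeleteItem, bound on BeginPlay to interaction completion, destroys the actor when that flag is set.
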(event OnComponentBeginOverlap(Sphere)
  (params (OverlappedComponent :type Primitive%20Component%20Object%20Reference) (OtherActor :type Actor%20Object%20Reference) (OtherComp :type Primitive%20Component%20Object%20Reference) (OtherBodyIndex :type Integer) (bFromSweep :type Boolean) (SweepResult :type Hit%20Result%20Structure%20%28by%20ref%29))
  (Utilities|Casting|CastToBP_Cat OtherActor)
  (Variables|Default|SetIsCatNear? true)
  (CallFunction|SetHighlight))

(event OnComponentEndOverlap(Sphere)
  (params (OverlappedComponent :type Primitive%20Component%20Object%20Reference) (OtherActor :type Actor%20Object%20Reference) (OtherComp :type Primitive%20Component%20Object%20Reference) (OtherBodyIndex :type Integer))
  (Utilities|Casting|CastToBP_Cat OtherActor)
  (Variables|Default|SetIsCatNear? false)
  (CallFunction|SetHighlight))

(event Custom|DeleteItem
  (if (Variables|Default|GetInterractionCompleted?)
    (Actor|DestroyActor)))

(event EventBeginPlay
  (EventDispatchers|BindEventtoInterractionCompleted (delegate Custom|DeleteItem)))

(fn ConstructionScript)

(fn SetHighlight
  (if (Variables|Default|GetIsCatNear?)
    (Rendering|Material|SetMaterial (Variables|Default|GetPaperSprite) 0 "/Game/InterractableObjects/key/Emission.Emission")
    (else
      (Rendering|Material|SetMaterial (Variables|Default|GetPaperSprite) 0 0))))

(fn Interract
  (params (Cat :type BP%20Cat%20Object%20Reference))
  (Development|PrintString (Utilities|GetDisplayName self))
  (Variables|Default|SetInterractionCompleted? true)
  (return self))