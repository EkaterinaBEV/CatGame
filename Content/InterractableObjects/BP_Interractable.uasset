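; Interactable pickup with a Paper2D sprite that highlights near the cat pawn and is destroyed once collected.
; Each Tick, a sphere trace for pawns caches the BP_Cat, swaps the sprite to an emissive material and manages a WB_Hints widget.
; Interract sets a completion flag, which Tick broadcasts through InterractionCompleted to DeleteItem.
; DeleteItem adds the actor to the GameInstance's collected-pickup save data before destroying it.
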(event Custom|DeleteItem
  (if (Variables|Default|GetInterractionCompleted?)
    ;[1 1 1] To save the level condition
    (Utilities|Array|AddUnique (Variables|/Game/Levels/Level1/Level1SaveGame.Level1SaveGame_C|GetCollectedPickUps (Variables|/Game/Cat/MyGameInstance.MyGameInstance_C|GetLevelSaveData%20 (Variables|/Game/Cat/BP_Cat.BP_Cat_C|GetAs%20My%20Game%20Instance (Variables|Default|GetCat)))) self)
    (Actor|DestroyActor)))

(event EventBeginPlay
  (EventDispatchers|BindEventtoInterractionCompleted (delegate Custom|DeleteItem)))

(event EventTick
  (params (DeltaSeconds :type Float%20%28single-precision%29))
  (CallFunction|SetHighlight)
  (if (Variables|Default|GetInterractionCompleted?)
    (Default|CallInterractionCompleted)))

(fn ConstructionScript)

(fn SetHighlight
  (bind _returnvalue (Transformation|GetActorLocation))
  (bind (_outhit _returnvalue_2) (Collision|SphereTraceForObjects _returnvalue (+ _returnvalue (* (Transformation|GetActorForwardVector) (Math|Vector|MakeVector 2e+02 0.0 0.0))) (Variables|Default|GetHighlightRadius) (Utilities|Array|MakeArray "ObjectTypeQuery3") false (Utilities|Array|MakeArray self) "None"))
  (if _returnvalue_2
    (bind _asbp_cat (Utilities|Casting|CastToBP_Cat (.HitActor (Collision|BreakHitResult _outhit))))
    (Variables|Default|SetCat _asbp_cat)
    (Rendering|Material|SetMaterial (Variables|Default|GetPaperSprite) 0 "/Game/InterractableObjects/key/Emission.Emission")
    (Utilities|IsValid (Variables|Default|GetHintWidget)
      (:Is%20Not%20Valid
        (bind _returnvalue_3 (UserInterface|CreateWidget "/Game/UI/UI_Level1/WB_Hints.WB_Hints_C" 0 (Variables|Default|GetText)))
        (bind _output_get (Variables|Default|SetHintWidget _returnvalue_3))
        (UserInterface|Viewport|AddtoViewport _output_get 0)))
    (else
      (Rendering|Material|SetMaterial (Variables|Default|GetPaperSprite) 0 0)
      (Utilities|IsValid (Variables|Default|GetHintWidget)
        (:Is%20Valid
          (Widget|RemovefromParent (Variables|Default|GetHintWidget)))))))

(fn Interract
  (params (Cat :type BP%20Cat%20Object%20Reference))
  (Development|PrintString (Utilities|GetDisplayName self))
  (Variables|Default|SetInterractionCompleted? true)
  (return self))