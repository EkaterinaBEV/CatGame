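; BP_PigeonScull is an interactable pigeon skull object that the cat can pick up.
; Its Interract function adds the skull to the interacting cat's inventory, sets InterractionCompleted and returns itself.
; The event graph holds only disabled default events, and the construction script just calls its parent.
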(event EventBeginPlay
  (|CallParentFunction) ; This node is disabled and will not be called.\nDrag off pins to build functionality.
)

(event Collision|EventActorBeginOverlap
  (params (OtherActor :type Actor%20Object%20Reference)))

(event EventTick
  (params (DeltaSeconds :type Float%20%28single-precision%29))
  (|CallParentFunction DeltaSeconds) ; This node is disabled and will not be called.\nDrag off pins to build functionality.
)

(fn ConstructionScript
  (|CallParentFunction))

(fn Interract
  (params (Cat :type BP%20Cat%20Object%20Reference))
  (Default|AddtoInv (Variables|/Game/Cat/BP_Cat.BP_Cat_C|GetInventory Cat) self)
  (Variables|Default|SetInterractionCompleted? true)
  (return self))