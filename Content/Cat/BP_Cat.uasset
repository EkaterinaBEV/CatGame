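; Player-controlled 2D side-scrolling cat character with sprinting, jumping, wall sliding, melee attack and item interaction.
; Tick picks the flipbook and capsule radius from movement state, flips controller yaw for facing, and line-traces forward while falling to enable wall slides and launched wall jumps.
; Attacks apply damage through a delayed line trace, while received damage lowers health, shakes the camera and updates HUD lives.
; Interaction sphere-traces for BP_Iterractable actors and adds to the inventory.
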(event Custom|UpdateAnimation
  ;[1 1 1] Animation
  (if (AI|Components|NavMovement|IsFalling (Variables|Character|GetCharacterMovement))
    (Components|Capsule|SetCapsuleRadius (Variables|Collision|GetCapsuleComponent) 1.0 true)
    (if (Variables|Checks|GetWallSlide?)
      (Sprite|SetFlipbook (Variables|Default|GetSprite) (Variables|Animation|GetWallSlide))
      (else
        (Sprite|SetFlipbook (Variables|Default|GetSprite) (select (< (.z (Transformation|GetVelocity)) 0.0) (Variables|Animation|GetDown) (Variables|Animation|GetUp)))))
    (else
      (Components|Capsule|SetCapsuleRadius (Variables|Collision|GetCapsuleComponent) 1.2e+02 true)
      (if (Variables|Checks|GetIsSprinting?)
        (Sprite|SetFlipbook (Variables|Default|GetSprite) (Variables|Animation|GetSprinting))
        (elif (Variables|Checks|GetIsAttacking?)
          (Sprite|SetFlipbook (Variables|Default|GetSprite) (Variables|Animation|GetAttacking))
          (else
            (Sprite|SetFlipbook (Variables|Default|GetSprite) (select (> (Math|Vector|VectorLength (Transformation|GetVelocity)) 0.0) (Variables|Animation|GetRun) (Variables|Animation|GetIdle)))))))))

(event Custom|WallSlideMech
  (bind _returnvalue (Transformation|GetActorLocation))
  ;[1 1 1] WallSlide
  (if (AI|Components|NavMovement|IsFalling (Variables|Character|GetCharacterMovement))
    (bind _outhit (Collision|LineTraceByChannel _returnvalue (+ _returnvalue (* (Transformation|GetActorForwardVector) (Math|Vector|MakeVector 5.0 0.0 0.0))) "TraceTypeQuery1" false 0 "ForDuration"))
    (Variables|Checks|SetWallSlide? (.bBlockingHit (Collision|BreakHitResult _outhit)))
    (else
      (Variables|Checks|SetWallSlide? false))))

(event Game|Damage|EventAnyDamage
  (params (Damage :type Float%20%28single-precision%29) (DamageType :type Damage%20Type%20Object%20Reference) (InstigatedBy :type Controller%20Object%20Reference) (DamageCauser :type Actor%20Object%20Reference))
  ;[1 1 1] WhenDamaged
  (Variables|Health|SetHealth (- (Variables|Health|GetHealth) Damage))
  (Camera|PlayWorldCameraShake "/Game/Cat/CamShake_CatDamage.CamShake_CatDamage_C" (Transformation|GetActorLocation) 0.0 1e+03)
  (for _index (range 1 (Math|Float|Truncate Damage))
    (Default|SetLives (Variables|Default|GetPlayerHUD))))

(event EventTick
  (params (DeltaSeconds :type Float%20%28single-precision%29))
  (bind _returnvalue (Pawn|GetController))
  (bind _returnvalue_2 (Pawn|GetController))
  (CallFunction|UpdateAnimation)
  (CallFunction|WallSlideMech)
  (if (not (Variables|Checks|GetWallSlide?))
    ;[1 1 1] Rotation
    (Math|Float|CompareFloat (.x (Variables|/Script/Engine.MovementComponent|GetVelocity (Variables|Character|GetCharacterMovement))) 0.0
      (:>
        (Utilities|IsValid _returnvalue_2 :!label _label
          (:Is%20Valid
            (Pawn|SetControlRotation _returnvalue_2 (Math|Rotator|MakeRotator 0.0 0.0 0.0)))))
      (:==
        (if (Variables|Checks|GetIsMovingRIght?)
          (goto _label)
          (else
            (Utilities|IsValid _returnvalue :!label _label_2
              (:Is%20Valid
                (Pawn|SetControlRotation _returnvalue (Math|Rotator|MakeRotator 0.0 0.0 1.8e+02)))))))
      (:<
        (goto _label_2)))))

(event EventBeginPlay
  (Variables|/Script/Engine.CharacterMovementComponent|SetMaxWalkSpeed (Variables|Character|GetCharacterMovement) (Variables|Default|GetCatSpeed))
  (bind _returnvalue (UserInterface|CreateWidget "/Game/UI/HUD/PlayerHUD.PlayerHUD_C"))
  (bind _output_get (Variables|Default|SetPlayerHUD _returnvalue))
  (UserInterface|Viewport|AddtoViewport _output_get 0))

(event Input|ActionEvents|InputActionJump
  (params (Key :type Key%20Structure :default "None"))
  ;[1 1 1] HandleInput
  (:Pressed
    (if (not (Variables|Checks|GetIsAttacking?))
      (if (Variables|Checks|GetWallSlide?)
        (Character|LaunchCharacter (Math|Vector|MakeVector (* (.x (Transformation|GetActorForwardVector)) -1.5e+03) 0.0 6.5e+02) true true)
        (else
          (Character|Jump)))))
  (:Released
    (Character|StopJumping)))

(event Input|ActionEvents|InputActionSprint
  (params (Key :type Key%20Structure :default "None"))
  ;[1 1 1] HandleInput
  (:Pressed
    (if (not (Variables|Checks|GetIsAttacking?))
      (Variables|/Script/Engine.CharacterMovementComponent|SetMaxWalkSpeed (Variables|Character|GetCharacterMovement) (Variables|Default|GetSprintingSpeed))
      (Variables|Checks|SetIsSprinting? true)))
  (:Released
    (Variables|/Script/Engine.CharacterMovementComponent|SetMaxWalkSpeed (Variables|Character|GetCharacterMovement) (Variables|Default|GetCatSpeed))
    (Variables|Checks|SetIsSprinting? false)))

(event Input|ActionEvents|InputActionMeleeAttack
  (params (Key :type Key%20Structure :default "None"))
  (bind _returnvalue (Transformation|GetActorLocation))
  ;[1 1 1] MeleeAttack
  (:Pressed
    (if (not (or (Variables|Checks|GetWallSlide?) (AI|Components|NavMovement|IsFalling (Variables|Character|GetCharacterMovement))))
      (Variables|Checks|SetIsAttacking? true)
      (Utilities|FlowControl|Delay 0.4)
      (Utilities|FlowControl|Sequence
        (:then_0
          (Variables|Checks|SetIsAttacking? false))
        (:then_1
          (bind _outhit (Collision|LineTraceForObjects _returnvalue (+ _returnvalue (* (Transformation|GetActorForwardVector) (Math|Vector|MakeVector 2e+02 0.0 0.0))) (Utilities|Array|MakeArray "ObjectTypeQuery3") false (Utilities|Array|MakeArray self) "ForDuration"))
          (Development|PrintString (Utilities|GetDisplayName (.HitActor (Collision|BreakHitResult _outhit))))
          (Game|Damage|ApplyDamage (.HitActor (Collision|BreakHitResult _outhit)) 1.0 0 self))))))

(event Input|ActionEvents|InputActionInterract
  (params (Key :type Key%20Structure :default "None"))
  (bind _scene (Variables|Default|GetScene))
  (bind _returnvalue (Transformation|GetWorldLocation _scene))
  ;[1 1 1] Interraction
  (:Pressed
    (bind _outhit (Collision|SphereTraceByChannel _returnvalue (+ _returnvalue (* (Transformation|GetActorForwardVector) (Math|Vector|MakeVector 2e+02 0.0 0.0))) 1e+02 "TraceTypeQuery1" false (Utilities|Array|MakeArray self) "ForDuration"))
    (bind _asbp_iterractable (Utilities|Casting|CastToBP_Iterractable (.HitActor (Collision|BreakHitResult _outhit)))
      (:then
        (bind _object (Default|Interract _asbp_iterractable self))
        (Variables|Default|SetObject _object)
        (Variables|Checks|SetInterractionSuccess true)
        (Default|AddtoInventory (Variables|Default|GetInventory)))
      (:CastFailed
        (Development|PrintString "Failed")
        (Variables|Default|SetObject 0)
        (Variables|Checks|SetInterractionSuccess false)))))

(event Input|ActionEvents|InputActionInventory
  (params (Key :type Key%20Structure :default "None"))
  (:Pressed
    (for _array_element (Variables|/Game/Cat/Cat_Inventory.Cat_Inventory_C|GetItemsAvailable (Variables|Default|GetInventory))
      (Development|PrintString (Utilities|GetDisplayName _array_element) true true "(R=0.038336,G=0.816000,B=0.000000,A=1.000000)"))))

(event Input|AxisEvents|InputAxisMoveRIght
  (params (AxisValue :type Float%20%28single-precision%29))
  ;[1 1 1] HandleInput
  (if (not (Variables|Checks|GetIsAttacking?))
    (if (> AxisValue 0.0)
      (Variables|Checks|SetIsMovingRIght? true)
      (elif (< AxisValue 0.0)
        (Variables|Checks|SetIsMovingRIght? false)))
    (Pawn|Input|AddMovementInput "1.000000, 0, 0" AxisValue false)))

(event Input|KeyboardEvents|1
  (params (Key :type Key%20Structure :default "None"))
  ;[1 1 1] WhenDamaged
  (:Pressed
    (Variables|Health|SetHealth (- (Variables|Health|GetHealth) (stale Game|Damage|EventAnyDamage Damage)))
    (Camera|PlayWorldCameraShake "/Game/Cat/CamShake_CatDamage.CamShake_CatDamage_C" (Transformation|GetActorLocation) 0.0 1e+03)
    (for _index (range 1 (Math|Float|Truncate (stale Game|Damage|EventAnyDamage Damage)))
      (Default|SetLives (Variables|Default|GetPlayerHUD)))))

(fn ConstructionScript)

(fn ChangeHealth)

(fn Interract
  (params (Cat :type BP%20Cat%20Object%20Reference)))